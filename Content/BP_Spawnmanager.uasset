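; BP_Spawnmanager is a wave manager that spawns enemies and checks when all are gone.
; A second after BeginPlay, SpawnEnemies spawns a BP_Enemy at the transform of every existing BP_Enemy, although its comment describes spawners.
; NewWaveCheck, meant to be called by dying enemies, counts remaining enemies and announces a new wave at zero.
; Its final delay leads nowhere, so no respawn follows.
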(event Custom|Spawn%20Enemies
  (bind _outactors (Actor|GetAllActorsOfClass "/Game/BP_Enemy.BP_Enemy_C"))
  (for _array_element _outactors
    (Development|PrintString (Utilities|GetDisplayName _array_element))
    (if true
      (Game|SpawnActorfromClass "/Game/BP_Enemy.BP_Enemy_C" (Transformation|GetWorldTransform (Variables|/Game/BP_Enemy.BP_Enemy_C|GetDefaultSceneRoot _array_element)) "Undefined" "MultiplyWithRoot" 0 0))))

(event Custom|NewWaveCheck
  (Development|PrintString "Was that the last enemy?")
  (bind _outactors (Actor|GetAllActorsOfClass "/Game/BP_Enemy.BP_Enemy_C"))
  (if (> (Utilities|Array|Length _outactors) 0) ; Are there more than ZERO enemies?
    (Development|PrintString "You were not the last one.")
    (else
      (Development|PrintString "ENEMIES INCOMING" true true "(R=1.000000,G=0.000000,B=0.186981,A=1.000000)")
      (Utilities|FlowControl|Delay 3.0))))

(event EventBeginPlay
  (Development|PrintString "Spawn Manager exists.")
  (Utilities|FlowControl|Delay 1.0)
  (CallFunction|SpawnEnemies))

(fn ConstructionScript)